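; Actor component that tracks the player's score during gameplay.
; It resets the current score to zero on BeginPlay, and AddPoints increases it by a given amount.
; Each addition then calls CallEventAddPoints, apparently to notify listeners, and prints the new total on screen for debugging.
; GetScore exposes the current value to other Blueprints.
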(event `self.ReceiveBeginPlay`
  (set `self.CurrentScore` 0))

(fn `AddPoints`
  (params (Points :type Integer :default 20))
  (bind _output_get (set `self.CurrentScore` (+ Points (`self.CurrentScore`))))
  (`self.EventAddPoints`)
  (`KismetSystemLibrary.PrintString` (`KismetStringLibrary.Concat_StrStr` "Current Score : " (`KismetStringLibrary.Conv_IntToString` _output_get))))

(fn `GetScore`
  (returns (Score :type Integer))
  (return (`self.CurrentScore`)))