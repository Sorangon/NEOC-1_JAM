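; Base player controller that adds the game HUD on BeginPlay and tracks where the player aims with the mouse.
; Each tick it traces from the mouse into the world and stores the normalized 2D direction from the controlled pawn to the hit, exposed through GetAimDirection.
; Lose triggers EventDie on the possessed BP_Drone, and LandLauncher possesses the given launcher.
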(event `self.ReceiveBeginPlay`
  (bind _returnvalue (`|CreateWidget` "/Game/GameContent/UI/GameHUD/BP/WBP_GameHUD.WBP_GameHUD_C" self))
  (`UserWidget.AddToPlayerScreen` _returnvalue 0))

(event `self.ReceiveTick`
  (params (DeltaSeconds :type "Float (single-precision)"))
  (`self.SetAimDirection`))

(event `Event Lose`
  (bind _asbp_drone (cast `/Game/GameContent/Gameplay/Elements/Drone/BP/BP_Drone` (`self.K2_GetPawn`)))
  (`/Game/GameContent/Gameplay/Elements/Drone/BP/BP_Drone.Event Die` _asbp_drone))

(event `Event Land Launcher`
  (params (Launcher :type "/Game/GameContent/Gameplay/Elements/Launcher/BP/BP_Launcher Object Reference"))
  (`self.Possess` Launcher))

(fn `GetAimDirection`
  (returns (Direction :type "Vector2D Structure"))
  (return (`self._aimDirection`)))

(fn `SetAimDirection`
  (bind _returnvalue (`self.K2_GetPawn`))
  (`/Engine/EditorBlueprintResources/StandardMacros.IsValid` _returnvalue
    (:`Is Valid`
      (set `self._aimDirection` (`KismetMathLibrary.Normal2D` (`KismetMathLibrary.MakeVector2D` (.x (- (`/Game/GameContent/Generic/Blueprint/Libraries/BPLIB_MouseMethods.GetWorldToMouseRayHit` self "TraceTypeQuery3") (`self.K2_GetActorLocation` _returnvalue))) (.y (- (`/Game/GameContent/Generic/Blueprint/Libraries/BPLIB_MouseMethods.GetWorldToMouseRayHit` self "TraceTypeQuery3") (`self.K2_GetActorLocation` _returnvalue)))))))
    (:`Is Not Valid`
      (set `self._aimDirection` (0.0 0.0)))))

(fn `UserConstructionScript`)