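; BP_Collidable is a collidable enemy element that dies from any damage it takes.
; On BeginPlay it registers itself with the EnemiesManager held by BP_GameState.
; Any damage, regardless of amount, calls Die, which unregisters it from the manager, plays a 2D impact sound and destroys the actor.
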(event `self.ReceiveBeginPlay`
  (bind _asbp_game_state (cast `/Game/GameContent/Gameplay/Systems/GameStates/BP_GameState` (`GameplayStatics.GetGameState`)))
  (`/Game/GameContent/Gameplay/Elements/Collidables/Enemies/BP/BP_EnemiesManager.RegisterEnemy` (`/Game/GameContent/Gameplay/Systems/GameStates/BP_GameState.EnemiesManager` _asbp_game_state) self))

(event `self.ReceiveAnyDamage`
  (params (Damage :type "Float (single-precision)") (DamageType :type "DamageType Object Reference") (InstigatedBy :type "Controller Object Reference") (DamageCauser :type "Actor Object Reference"))
  (`self.Die`))

(fn `Die`
  (bind _asbp_game_state (cast `/Game/GameContent/Gameplay/Systems/GameStates/BP_GameState` (`GameplayStatics.GetGameState`)))
  (`/Game/GameContent/Gameplay/Elements/Collidables/Enemies/BP/BP_EnemiesManager.UnregisterEnemy` (`/Game/GameContent/Gameplay/Systems/GameStates/BP_GameState.EnemiesManager` _asbp_game_state) self)
  (`GameplayStatics.PlaySound2D` "/Game/GameContent/Gameplay/Elements/Collidables/Enemies/SFX/SFX_CollidableImpact.SFX_CollidableImpact" 1.0 1.0 0.0 null null)
  (`self.K2_DestroyActor`))

(fn `UserConstructionScript`)