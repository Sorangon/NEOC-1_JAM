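; Enemy spawner actor that places each wave's actors at designated spawn points in the level.
; On BeginPlay it registers itself as the Spawner on the EnemiesManager held by BP_GameState.
; SpawnWave loops over a wave's entries and spawns each collidable actor class at the location of the SpawnPoints element indexed by its spawner ID.
; Spawns use zero rotation and unit scale, adjusting for collisions but always spawning.
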(event `self.ReceiveBeginPlay`
  (bind _asbp_game_state (cast `/Game/GameContent/Gameplay/Systems/GameStates/BP_GameState` (`GameplayStatics.GetGameState`)))
  (set `/Game/GameContent/Gameplay/Elements/Ennemies/Test/BP/BP_EnemiesManager.Spawner` self (`/Game/GameContent/Gameplay/Systems/GameStates/BP_GameState.EnemiesManager` _asbp_game_state)))

(fn `SpawnWave`
  (params (Wave :type "/Game/GameContent/Gameplay/Datas/DataStructs/WaveData Structure"))
  (for _array_element Wave_Object_12_E03316F3487276810D29BC8FB669E6AF
    (`|SpawnActorFromClass` (break `/Game/GameContent/Gameplay/Datas/DataStructs/EnemyData` _array_element) (`KismetMathLibrary.MakeTransform` (`self.K2_GetActorLocation` (`|GetArrayItem` (`self.SpawnPoints`) (`.SpawnerID_5_46C5F1BE421DC32B88AE3AA75FC738B1` (break `/Game/GameContent/Gameplay/Datas/DataStructs/EnemyData` _array_element))))) "AdjustIfPossibleButAlwaysSpawn" "OverrideRootScale" null null)))

(fn `UserConstructionScript`)