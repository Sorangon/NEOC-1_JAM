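; Test enemy manager that runs the rounds and waves of Level1, loaded from the DT_Levels data table on BeginPlay.
; Timers delay each round and follow-up wave, and the Spawner spawns each wave from the level data.
; Enemies register in a tracked list; each removal checks the count against the wave's allowed remainder to advance waves, then rounds.
; Progress and the final win are only reported through debug prints.
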(event `self.ReceiveBeginPlay`
  (bind _returnvalue (`|GetDataTableRow` "/Game/GameContent/Gameplay/Datas/GameDatas/DT_Levels.DT_Levels" "Level1")
    (:`then`
      (set `self._currentLevel` _returnvalue)
      (set `self._currentRoundID` 0)
      (`KismetSystemLibrary.K2_SetTimerDelegate` (delegate `On Start Round`) 2.0))))

(event `On Start Round`
  (`KismetSystemLibrary.PrintString` (`KismetStringLibrary.Concat_StrStr` "Starting round : " (`KismetStringLibrary.Conv_IntToString` (`self._currentRoundID`))))
  (set `self._currentWaveID` 0)
  (`self.On Wave Ready`))

(event `On Round Over`
  (`KismetSystemLibrary.PrintString` (`KismetStringLibrary.Concat_StrStr` "Round " (`KismetStringLibrary.Conv_IntToString` (`self._currentRoundID`)) " Cleared"))
  (bind _result (`/Engine/EditorBlueprintResources/StandardMacros.IncrementInt` (`self._currentRoundID`))
    (:`  `
      (if (< _result (`KismetArrayLibrary.Array_Length` (`.Rounds_5_63A196A347DCED14314543BCB7DDE7E5` (break `/Game/GameContent/Gameplay/Datas/DataStructs/LevelData` (`self._currentLevel`)))))
        (`KismetSystemLibrary.K2_SetTimerDelegate` (delegate `On Start Round`) 2.0)
        (else
          (`KismetSystemLibrary.PrintString` "Game won !" true true (struct :`G` 1.0 :`B` 0.268722 :`A` 1.0)))))))

(event `On Wave Ready`
  (`KismetSystemLibrary.PrintString` (`KismetStringLibrary.Concat_StrStr` "Starting Wave : " (`KismetStringLibrary.Conv_IntToString` (`self._currentWaveID`))))
  (`/Game/GameContent/Gameplay/Elements/Spawner/BP_EnemiesSpawner.SpawnWave` (`self.Spawner`) (`|GetArrayItem` (`.Waves_3_6F1A49844C77F85552F58E9A10940B2E` (break `/Game/GameContent/Gameplay/Datas/DataStructs/RoundData` (`|GetArrayItem` (`.Rounds_5_63A196A347DCED14314543BCB7DDE7E5` (break `/Game/GameContent/Gameplay/Datas/DataStructs/LevelData` (`self._currentLevel`))) (`self._currentRoundID`)))) (`self._currentWaveID`))))

(event `On Wave Over`
  (bind _result (`/Engine/EditorBlueprintResources/StandardMacros.IncrementInt` (`self._currentWaveID`))
    (:`  `
      (if (< _result (`KismetArrayLibrary.Array_Length` (`.Waves_3_6F1A49844C77F85552F58E9A10940B2E` (break `/Game/GameContent/Gameplay/Datas/DataStructs/RoundData` (`|GetArrayItem` (`.Rounds_5_63A196A347DCED14314543BCB7DDE7E5` (break `/Game/GameContent/Gameplay/Datas/DataStructs/LevelData` (`self._currentLevel`))) (`self._currentRoundID`))))))
        (`KismetSystemLibrary.K2_SetTimerDelegate` (delegate `On Wave Ready`) 2.0)
        (else
          (`self.On Round Over`))))))

(fn `CheckWaveState`
  (if (<= (`KismetArrayLibrary.Array_Length` (`self._spawedCollidables`)) (`.AllowedRemainingEnnemis_16_B9809A5B460B8F4419AD979AD840724B` (break `/Game/GameContent/Gameplay/Datas/DataStructs/WaveData` (`|GetArrayItem` (`.Waves_3_6F1A49844C77F85552F58E9A10940B2E` (break `/Game/GameContent/Gameplay/Datas/DataStructs/RoundData` (`|GetArrayItem` (`.Rounds_5_63A196A347DCED14314543BCB7DDE7E5` (break `/Game/GameContent/Gameplay/Datas/DataStructs/LevelData` (`self._currentLevel`))) (`self._currentRoundID`)))) (`self._currentWaveID`)))))
    (`KismetSystemLibrary.PrintString` (`KismetStringLibrary.Concat_StrStr` "Wave " (`KismetStringLibrary.Conv_IntToString` (`self._currentWaveID`)) " Cleared"))
    (`self.On Wave Over`)))

(fn `RegisterEnemy`
  (params (Enemy :type "/Game/GameContent/Gameplay/Elements/Ennemies/Test/BP/BP_TEstEnemy Object Reference"))
  (`KismetArrayLibrary.Array_Add` (`self._spawedCollidables`) Enemy))

(fn `UnregisterEnemy`
  (params (Enemy :type "/Game/GameContent/Gameplay/Elements/Ennemies/Test/BP/BP_TEstEnemy Object Reference"))
  (`KismetArrayLibrary.Array_RemoveItem` (`self._spawedCollidables`) Enemy)
  (`self.CheckWaveState`)
  (return))