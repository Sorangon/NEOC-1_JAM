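; BP_AttractorsManager is a manager component that keeps a registry of attractor elements in the game.
; RegisterAttractor adds an attractor to the list, prints the new count for debugging, and fires an attractor-registered event dispatcher.
; GetAttractors returns the current list to callers.
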(fn `GetAttractors`
  (returns (Attractors :type "Array of Attractor Object Reference"))
  (return (`self._attractors`)))

(fn `RegisterAttractor`
  (params (Attractor :type "Attractor Object Reference"))
  (`KismetArrayLibrary.Array_Add` (`self._attractors`) Attractor)
  (`KismetSystemLibrary.PrintString` (`KismetStringLibrary.Concat_StrStr` "Registered attractor, now containing : " (`KismetStringLibrary.Conv_IntToString` (`KismetArrayLibrary.Array_Length` (`self._attractors`)))))
  (`self.OnAttractorRegitered`))