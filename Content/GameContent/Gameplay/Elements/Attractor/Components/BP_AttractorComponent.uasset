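; Attractor component that registers with the game state's attractor manager on BeginPlay and unregisters on EndPlay.
; It supplies the target direction for an attached object, using that object's position, direction and speed.
; The direction is the horizontal tangent around the attractor, signed by a dot product to follow the object's current travel, giving an orbit in either sense.
; The result is scaled to the object's speed, with no speed bonus.
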(event `self.ReceiveBeginPlay`
  (`self.RegisterToManager`))

(event `self.ReceiveEndPlay`
  (params (EndPlayReason :type "EEndPlayReason Enum" :default "Destroyed"))
  (`self.UnregisterToManager`))

(fn `GetAttachedObjectTargetDirection`
  (params (ObjectPosition :type "Vector Structure") (ObjectDirection :type "Vector Structure") (ObjectSpeed :type "Float (double-precision)"))
  (returns (Direction :type "Vector Structure") (SpeedBonus :type "Float (double-precision)"))
  (bind _returnvalue (`KismetMathLibrary.Cross_VectorVector` (- (`self.K2_GetComponentLocation`) ObjectPosition) (`KismetMathLibrary.Vector_Up`)))
  (return (* (`KismetMathLibrary.Normal` (* _returnvalue (`KismetMathLibrary.Dot_VectorVector` _returnvalue ObjectDirection))) ObjectSpeed) 0.0))

(fn `RegisterToManager`
  (bind _asbp_game_state (cast `/Game/GameContent/Gameplay/Systems/GameStates/BP_GameState` (`GameplayStatics.GetGameState`)))
  (`/Game/GameContent/Gameplay/Elements/Attractor/Components/BP_AttractorsManager.RegisterAttractor` (`/Game/GameContent/Gameplay/Systems/GameStates/BP_GameState.GetAttractorManager` _asbp_game_state) self))

(fn `UnregisterToManager`
  (bind _asbp_game_state (cast `/Game/GameContent/Gameplay/Systems/GameStates/BP_GameState` (`GameplayStatics.GetGameState`)))
  (`/Game/GameContent/Gameplay/Elements/Attractor/Components/BP_AttractorsManager.UnregisterAttractor` (`/Game/GameContent/Gameplay/Systems/GameStates/BP_GameState.GetAttractorManager` _asbp_game_state) self))