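; BP_GameplayCamera is a gameplay camera actor that shifts its view to follow the player's pawn relative to a fixed Center point.
; Each tick it takes the pawn's horizontal offset from Center, scales it by DistanceMultiplier and uses that as the camera component's target relative location.
; The camera eases toward that target with a frame-time lerp whose speed is set by Damping.
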(event `self.ReceiveTick`
  (params (DeltaSeconds :type "Float (single-precision)"))
  (bind _returnvalue (`Controller.K2_GetPawn` (`GameplayStatics.GetPlayerController` 0)))
  (`/Engine/EditorBlueprintResources/StandardMacros.IsValid` _returnvalue
    (:`Is Valid`
      (`SceneComponent.K2_SetRelativeLocation` (`self.CameraComponent`) (`KismetMathLibrary.VLerp` (`SceneComponent.RelativeLocation` (`self.CameraComponent`)) (* (* (- (`self.K2_GetActorLocation` _returnvalue) (`self.K2_GetActorLocation` (`self.Center`))) (1.0 1.0 0.0)) (`self.DistanceMultiplier`)) (* DeltaSeconds (/ 1.0 (`self.Damping`)))) false false))))

(fn `UserConstructionScript`)