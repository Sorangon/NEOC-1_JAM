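; Grappling component that picks and latches onto attractors or walls in the owning pawn's aim direction, exposing grab state for other code.
; Each tick it filters the GameState manager's attractors by range, then targets the best aim-aligned one via dot-product threshold.
; Grab locks the target's position, falling back to a line trace; deploy and release play sounds.
; Range, target and rope render only as debug shapes.
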(event `self.ReceiveBeginPlay`
  (`|ExecutionSequence`
    (:`then_0`
      ;[1 1 1] Get Owner controller
      (bind _aspawn (cast `Pawn` (`self.GetOwner`)))
      (bind _asbp_base_controller (cast `/Game/GameContent/Gameplay/Elements/PlayerController/BP_BaseController` (`Pawn.GetController` _aspawn)))
      (set `self._playerController` _asbp_base_controller))
    (:`then_1`
      ;[1 1 1] Get Attractors Manager
      (bind _asbp_game_state (cast `/Game/GameContent/Gameplay/Systems/GameStates/BP_GameState` (`GameplayStatics.GetGameState`)))
      (set `self._attractorsManager` (`/Game/GameContent/Gameplay/Systems/GameStates/BP_GameState.GetAttractorManager` _asbp_game_state)))))

(event `self.ReceiveTick`
  (params (DeltaSeconds :type "Float (single-precision)"))
  (bind __targetattractor (`self._targetAttractor`))
  (bind _returnvalue (`Actor.K2_GetActorLocation` (`self.GetOwner`)))
  (`|ExecutionSequence`
    (:`then_0`
      ;[1 1 1] Display Range
      (`KismetSystemLibrary.DrawDebugCircle` _returnvalue (- (`self.Detection Range`) 50.0) 40 (struct :`R` 0.569702 :`G` 1.0 :`B` 0.463061 :`A` 1.0) 0.0 5.0 (1.0 0.0 0.0) (0.0 1.0 0.0))
      (if (`self._isGrabbing`)
        (`KismetSystemLibrary.DrawDebugLine` _returnvalue (`self._grabbedPosition`) (struct :`R` 0.026724 :`G` 0.31226 :`B` 1.0 :`A` 1.0) 0.0 20.0)))
    (:`then_1`
      (`self.FindNearAttractors`)
      (`self.FindTargetAttractor`)
      (`/Engine/EditorBlueprintResources/StandardMacros.IsValid` __targetattractor
        (:`Is Valid`
          (`KismetSystemLibrary.DrawDebugSphere` (`SceneComponent.K2_GetComponentLocation` __targetattractor) 200.0 12 (struct :`R` 1.0 :`B` 0.790003 :`A` 1.0) 0.0 10.0))))))

(fn `DisplayNearAttractors`
  (locals (ActorLocation :type "Vector Structure"))
  (set `local.ActorLocation` (`Actor.K2_GetActorLocation` (`self.GetOwner`)))
  (for _array_element (`self._nearAttractorsID`)
    (`KismetSystemLibrary.DrawDebugLine` (`local.ActorLocation`) (`SceneComponent.K2_GetComponentLocation` (`|GetArrayItem` (`/Game/GameContent/Gameplay/Elements/Attractor/Components/BP_AttractorsManager.GetAttractors` (`self._attractorsManager`)) _array_element)) (struct :`R` 0.410376 :`G` 1.0 :`B` 0.430083 :`A` 0.05) (`self.GetComponentTickInterval`) 5.0)))

(fn `FindNearAttractors`
  (locals (ActorLocation :type "Vector Structure") (SqrRange :type "Float (double-precision)") (NearAttractors :type "Array of Integer"))
  (set `local.ActorLocation` (`Actor.K2_GetActorLocation` (`self.GetOwner`)))
  (set `local.SqrRange` (* (`self.Detection Range`) (`self.Detection Range`)))
  (`KismetArrayLibrary.Array_Clear` (`self._nearAttractorsID`)) ; Clear the near attractorts array
  (for (_array_element _array_index) (`/Game/GameContent/Gameplay/Elements/Attractor/Components/BP_AttractorsManager.GetAttractors` (`self._attractorsManager`))
    ;[1 1 1] Check if attractor is near enough and adds it to the list if it's the case
    (if (<= (`KismetMathLibrary.Vector_DistanceSquared` (`SceneComponent.K2_GetComponentLocation` _array_element) (`local.ActorLocation`)) (`local.SqrRange`))
      (`KismetArrayLibrary.Array_Add` (`self._nearAttractorsID`) _array_index))))

(fn `FindTargetAttractor`
  (locals (AimDirection :type "Vector Structure") (SmallestDot :type "Float (double-precision)") (ClosestAttractor :type "Attractor Object Reference") (DotThreshold :type "Float (double-precision)"))
  (set `local.AimDirection` (`KismetMathLibrary.Conv_Vector2DToVector` (`/Game/GameContent/Gameplay/Elements/PlayerController/BP_BaseController.GetAimDirection` (`self._playerController`))))
  (set `local.DotThreshold` (/ (- (`self.CursorAngleThreshold`) 90.0) 90.0))
  (for _array_element (`self._nearAttractorsID`)
    (bind _output (`|GetArrayItem` (`/Game/GameContent/Gameplay/Elements/Attractor/Components/BP_AttractorsManager.GetAttractors` (`self._attractorsManager`)) _array_element))
    (bind _returnvalue (`KismetMathLibrary.Dot_VectorVector` (`KismetMathLibrary.Normal` (- (`Actor.K2_GetActorLocation` (`self.GetOwner`)) (`SceneComponent.K2_GetComponentLocation` _output))) (`local.AimDirection`)))
    (if (and (< _returnvalue (`local.SmallestDot`)) (<= _returnvalue (`local.DotThreshold`)))
      (set `local.SmallestDot` _returnvalue)
      (set `local.ClosestAttractor` _output)))
  (set `self._targetAttractor` (`local.ClosestAttractor`)))

(fn `GetGrabInfos`
  (returns (IsGrabbing :type Boolean) (GrabbedPosition :type "Vector Structure") (GrabbedAttractor :type "Attractor Object Reference"))
  (return (`self._isGrabbing`) (`self._grabbedPosition`) (`self._targetAttractor`)))

(fn `Grab`
  (returns (Success :type Boolean) (HasGrabbedAttractor :type Boolean) (Attractor :type "Attractor Object Reference") (_targetAttractor :type "Attractor Object Reference"))
  (bind __targetattractor (`self._targetAttractor`))
  (bind _returnvalue (`Actor.K2_GetActorLocation` (`self.GetOwner`)))
  ;[1 1 1] Check if the player targets an attractor
  (`/Engine/EditorBlueprintResources/StandardMacros.IsValid` __targetattractor
    (:`Is Valid`
      ;[1 1 1] Grab the attractor
      (set `self._isGrabbing` true)
      (`self.GrabFeedback`)
      (set `self._grabbedPosition` (`SceneComponent.K2_GetComponentLocation` __targetattractor))
      (return true true null __targetattractor))
    (:`Is Not Valid`
      ;[1 1 1] Detect walls
      (bind (_outhit _returnvalue_2) (`KismetSystemLibrary.LineTraceSingle` :`Start` _returnvalue :`End` (+ (`KismetMathLibrary.Conv_Vector2DToVector` (* (`/Game/GameContent/Gameplay/Elements/PlayerController/BP_BaseController.GetAimDirection` (`self._playerController`)) (`self.Detection Range`))) _returnvalue) :`TraceChannel` "TraceTypeQuery4" :`DrawTime` 0.5))
      (if _returnvalue_2
        (set `self._isGrabbing` true)
        (set `self._grabbedPosition` (`.ImpactPoint` (`GameplayStatics.BreakHitResult` _outhit)))
        (`self.GrabFeedback`)
        (return true false null null)
        (else
          ;[0.1927 0 0] Missed
          (return false false null null))))))

(fn `GrabbedPosition`
  (returns (GrabbedPosition :type "Vector Structure"))
  (return (`self._grabbedPosition`)))

(fn `GrabFeedback`
  (`GameplayStatics.PlaySound2D` "/Game/GameContent/Gameplay/Elements/Drone/SFX/SW_GrapplingDeploy.SW_GrapplingDeploy" 1.0 1.0 0.0 null null))

(fn `Ungrab`
  (set `self._isGrabbing` false)
  (`GameplayStatics.PlaySound2D` "/Game/GameContent/Gameplay/Elements/Drone/SFX/SW_GrapplingRelease.SW_GrapplingRelease" 1.0 1.0 0.0 null null))