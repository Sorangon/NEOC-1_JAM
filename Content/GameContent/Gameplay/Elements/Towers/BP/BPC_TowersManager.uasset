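; Blueprint component that keeps the registry of tower actors in the game.
; Registering or unregistering a tower updates the list, fires the matching event with the new count, and signals when the last tower is removed.
; Query functions return the count, the full list, or the tower nearest a position, found by a linear scan on squared distances.
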(fn `GetNearestTower`
  (params (Position :type "Vector Structure"))
  (returns (Tower :type "/Game/GameContent/Gameplay/Elements/Towers/BP/BP_Tower Object Reference"))
  (locals (NearestTower :type "/Game/GameContent/Gameplay/Elements/Towers/BP/BP_Tower Object Reference") (ClostestSqrDistance :type "Float (double-precision)" :default 6.873995514006733e+17) (IteratedSqrDistance :type "Float (double-precision)"))
  (for _array_element (`self._towers`)
    (bind _output_get (set `local.IteratedSqrDistance` (`KismetMathLibrary.Vector_DistanceSquared` (`Actor.K2_GetActorLocation` _array_element) Position)))
    (if (< _output_get (`local.ClostestSqrDistance`))
      (set `local.ClostestSqrDistance` (`local.IteratedSqrDistance`))
      (set `local.NearestTower` _array_element)))
  (return (`local.NearestTower`)))

(fn `GetTowers`
  (returns (Towers :type "Array of /Game/GameContent/Gameplay/Elements/Towers/BP/BP_Tower Object Reference"))
  (return (`self._towers`)))

(fn `GetTowersCount`
  (returns (Count :type Integer))
  (return (`KismetArrayLibrary.Array_Length` (`self._towers`))))

(fn `RegisterTower`
  (params (Tower :type "/Game/GameContent/Gameplay/Elements/Towers/BP/BP_Tower Object Reference"))
  (returns (TowersCount :type Integer))
  (locals (Towers :type Integer))
  (bind __towers (`self._towers`))
  (`KismetArrayLibrary.Array_Add` __towers Tower)
  (bind _output_get (set `local.Towers` (`KismetArrayLibrary.Array_Length` __towers)))
  (`self.OnTowerRegistered` _output_get)
  (return _output_get))

(fn `UnregisterTower`
  (params (Tower :type "/Game/GameContent/Gameplay/Elements/Towers/BP/BP_Tower Object Reference"))
  (returns (TowersRemaining :type Integer))
  (locals (RemainingTowers :type Integer))
  (bind __towers (`self._towers`))
  (bind _remainingtowers (`local.RemainingTowers`))
  (`KismetArrayLibrary.Array_RemoveItem` __towers Tower)
  (bind _output_get (set `local.RemainingTowers` (`KismetArrayLibrary.Array_Length` __towers)))
  (`self.OnTowerUnregistered` _output_get)
  (`|ExecutionSequence`
    (:`then_0`
      (if (<= _remainingtowers 0)
        (`self.OnTowersEmpty`)))
    (:`then_1`
      (return _remainingtowers))))