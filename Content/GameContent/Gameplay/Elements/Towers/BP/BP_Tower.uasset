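; BP_Tower is a tower actor with health that registers with the game state's TowersManager on begin play.
; A health component drives it: taking damage flashes a red debug sphere and updates the Fill parameter on a dynamic material of the health bar indicator.
; On death it unregisters from the manager and swaps its mesh to a dynamic material with a red emissive color.
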(event `self.ReceiveBeginPlay`
  (bind _healthbarindicator (`self.HealthBarIndicator`))
  (`|ExecutionSequence`
    (:`then_0`
      (`/Game/GameContent/Gameplay/Elements/Towers/BP/BPC_TowersManager.RegisterTower` (`/Game/GameContent/Gameplay/Systems/GameStates/BP_GameState.TowersManager` (cast `/Game/GameContent/Gameplay/Systems/GameStates/BP_GameState` (`GameplayStatics.GetGameState`) :!pure true)) self))
    (:`then_1`
      (bind _returnvalue (`PrimitiveComponent.CreateDynamicMaterialInstance` _healthbarindicator 0 (`PrimitiveComponent.GetMaterial` _healthbarindicator 0) "None"))
      (set `self._healthBarMaterial` _returnvalue))))

(event `self.HeathBar.OnDie`
  (bind _staticmesh (`self.StaticMesh`))
  (`/Game/GameContent/Gameplay/Elements/Towers/BP/BPC_TowersManager.UnregisterTower` (`/Game/GameContent/Gameplay/Systems/GameStates/BP_GameState.TowersManager` (cast `/Game/GameContent/Gameplay/Systems/GameStates/BP_GameState` (`GameplayStatics.GetGameState`) :!pure true)) self)
  (bind _returnvalue (`KismetMaterialLibrary.CreateDynamicMaterialInstance` (`PrimitiveComponent.GetMaterial` _staticmesh 0)))
  (`MaterialInstanceDynamic.SetVectorParameterValue` _returnvalue "Emissive Color" (struct :`R` 0.973958 :`B` 0.025591 :`A` 1.0))
  (`PrimitiveComponent.SetMaterial` _staticmesh 0 _returnvalue))

(event `self.HeathBar.OnTakeDamages`
  (params (`Lost Health` :type Integer))
  ;[1 1 1] Take damages
  (`KismetSystemLibrary.DrawDebugSphere` (`self.K2_GetActorLocation`) 150.0 20 (struct :`R` 1.0 :`B` 0.03671 :`A` 1.0) 0.2)
  (`MaterialInstanceDynamic.SetScalarParameterValue` (`self._healthBarMaterial`) "Fill" (`/Game/GameContent/Gameplay/Elements/Health/BPC_HeathBar.GetHealthPercentage` (`self.HeathBar`))))

(fn `UserConstructionScript`)