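; Test enemy Blueprint that moves with FloatingPawnMovement, attacks towers and dies from any damage.
; It registers with the game state's EnemiesManager on spawn, and Die unregisters it, plays an impact sound and destroys it.
; Attack damages the target tower's health bar, while Collide applies incoming damage to itself and returns no bounce or return damage.
; Recall stops movement and destroys it after a short delay, without unregistering.
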(event `self.ReceiveBeginPlay`
  (`|ExecutionSequence`
    (:`then_0`
      (bind _asbp_game_state (cast `/Game/GameContent/Gameplay/Systems/GameStates/BP_GameState` (`GameplayStatics.GetGameState`)))
      (`/Game/GameContent/Gameplay/Elements/Enemies/Test/BP/BP_EnemiesManager.RegisterEnemy` (`/Game/GameContent/Gameplay/Systems/GameStates/BP_GameState.EnemiesManager` _asbp_game_state) self))))

(event `self.ReceiveAnyDamage`
  (params (Damage :type "Float (single-precision)") (DamageType :type "DamageType Object Reference") (InstigatedBy :type "Controller Object Reference") (DamageCauser :type "Actor Object Reference"))
  (`self.Die`))

(event `Event Recall`
  (`NavMovementComponent.StopActiveMovement` (`self.FloatingPawnMovement`))
  (`KismetSystemLibrary.Delay` 0.5)
  (`self.K2_DestroyActor`))

(fn `Attack`
  (params (`Target Tower` :type "/Game/GameContent/Gameplay/Elements/Towers/BP_Tower Object Reference"))
  (`/Game/GameContent/Gameplay/Elements/Health/BPC_HeathBar.TakeDamages` (`/Game/GameContent/Gameplay/Elements/Towers/BP_Tower.HeathBar` `Target Tower`) (`self.Damages`)))

(fn `Collide`
  (params (GivenDamages :type Integer))
  (returns (`Collision Infos` :type "/Game/GameContent/Gameplay/Elements/Interfaces/Collidable/CollisionInfos Structure"))
  (`GameplayStatics.ApplyDamage` self (`KismetMathLibrary.Conv_IntToDouble` GivenDamages))
  (return (make `/Game/GameContent/Gameplay/Elements/Interfaces/Collidable/CollisionInfos` false 0 self)))

(fn `Die`
  (bind _asbp_game_state (cast `/Game/GameContent/Gameplay/Systems/GameStates/BP_GameState` (`GameplayStatics.GetGameState`)))
  (`/Game/GameContent/Gameplay/Elements/Enemies/Test/BP/BP_EnemiesManager.UnregisterEnemy` (`/Game/GameContent/Gameplay/Systems/GameStates/BP_GameState.EnemiesManager` _asbp_game_state) self)
  (`GameplayStatics.PlaySound2D` "/Game/GameContent/Gameplay/Elements/Enemies/Test/SFX/SFX_CollidableImpact.SFX_CollidableImpact" 1.0 1.0 0.0 null null)
  (`self.K2_DestroyActor`))

(fn `UserConstructionScript`)