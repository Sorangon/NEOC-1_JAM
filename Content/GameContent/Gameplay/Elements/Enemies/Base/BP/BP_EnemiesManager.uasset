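; Enemy manager that runs the rounds and waves of Level1 from DT_Levels.
; Each wave goes to the Spawner, and a registry of spawned enemies clears it when removals bring the count within that wave's allowed remainder.
; Waves chain on short timers, while round end advances the index, prints a win after the last and broadcasts OnRoundOver without starting the next.
; RecallAllEnemies sends Stop to registered enemies' AI controllers.
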(event `self.ReceiveBeginPlay`
  (bind _returnvalue (`|GetDataTableRow` "/Game/GameContent/Gameplay/Datas/GameDatas/DT_Levels.DT_Levels" "Level1")
    (:`then`
      (set `self._currentLevel` _returnvalue)
      (set `self._currentRoundID` 0)
      (`KismetSystemLibrary.K2_SetTimerDelegate` (delegate `Event Start Round`) 2.0))))

(event `Event Start Round`
  (`KismetSystemLibrary.PrintString` (`KismetStringLibrary.Concat_StrStr` "Starting round : " (`KismetStringLibrary.Conv_IntToString` (`self._currentRoundID`))))
  (set `self._currentWaveID` 0)
  (`self.On Wave Ready`))

(event `Event On Round Over`
  (`|ExecutionSequence`
    (:`then_0`
      (`KismetSystemLibrary.PrintString` (`KismetStringLibrary.Concat_StrStr` "Round " (`KismetStringLibrary.Conv_IntToString` (`self._currentRoundID`)) " Cleared"))
      (bind _result (`/Engine/EditorBlueprintResources/StandardMacros.IncrementInt` (`self._currentRoundID`))
        (:`  `
          (if (not (< _result (`KismetArrayLibrary.Array_Length` (`.Rounds_5_63A196A347DCED14314543BCB7DDE7E5` (break `/Game/GameContent/Gameplay/Datas/DataStructs/LevelDataOld` (`self._currentLevel`))))))
            (`KismetSystemLibrary.PrintString` "Game won !" true true (struct :`G` 1.0 :`B` 0.268722 :`A` 1.0))))))
    (:`then_1`
      (`self.OnRoundOver`))))

(event `On Wave Ready`
  (`KismetSystemLibrary.PrintString` (`KismetStringLibrary.Concat_StrStr` "Starting Wave : " (`KismetStringLibrary.Conv_IntToString` (`self._currentWaveID`))))
  (`/Game/GameContent/Gameplay/Elements/Spawner/BP_EnemiesSpawner.SpawnWave` (`self.Spawner`) (`|GetArrayItem` (`.Waves_3_6F1A49844C77F85552F58E9A10940B2E` (break `/Game/GameContent/Gameplay/Datas/DataStructs/RoundDataOld` (`|GetArrayItem` (`.Rounds_5_63A196A347DCED14314543BCB7DDE7E5` (break `/Game/GameContent/Gameplay/Datas/DataStructs/LevelDataOld` (`self._currentLevel`))) (`self._currentRoundID`)))) (`self._currentWaveID`))))

(event `On Wave Over`
  (bind _result (`/Engine/EditorBlueprintResources/StandardMacros.IncrementInt` (`self._currentWaveID`))
    (:`  `
      (if (< _result (`KismetArrayLibrary.Array_Length` (`.Waves_3_6F1A49844C77F85552F58E9A10940B2E` (break `/Game/GameContent/Gameplay/Datas/DataStructs/RoundDataOld` (`|GetArrayItem` (`.Rounds_5_63A196A347DCED14314543BCB7DDE7E5` (break `/Game/GameContent/Gameplay/Datas/DataStructs/LevelDataOld` (`self._currentLevel`))) (`self._currentRoundID`))))))
        (`KismetSystemLibrary.K2_SetTimerDelegate` (delegate `On Wave Ready`) 2.0)
        (else
          (`self.Event On Round Over`))))))

(fn `CheckWaveState`
  (if (<= (`KismetArrayLibrary.Array_Length` (`self._spawedEnemies`)) (`.AllowedRemainingEnnemis_16_B9809A5B460B8F4419AD979AD840724B` (break `/Game/GameContent/Gameplay/Datas/DataStructs/WaveDataOld` (`|GetArrayItem` (`.Waves_3_6F1A49844C77F85552F58E9A10940B2E` (break `/Game/GameContent/Gameplay/Datas/DataStructs/RoundDataOld` (`|GetArrayItem` (`.Rounds_5_63A196A347DCED14314543BCB7DDE7E5` (break `/Game/GameContent/Gameplay/Datas/DataStructs/LevelDataOld` (`self._currentLevel`))) (`self._currentRoundID`)))) (`self._currentWaveID`)))))
    (`KismetSystemLibrary.PrintString` (`KismetStringLibrary.Concat_StrStr` "Wave " (`KismetStringLibrary.Conv_IntToString` (`self._currentWaveID`)) " Cleared"))
    (`self.On Wave Over`)))

(fn `RecallAllEnemies`
  (for _array_element (`self._spawedEnemies`)
    (bind _asbp_generic_aicontroller (cast `/Game/GameContent/Gameplay/Elements/Enemies/Base/BP/BP_GenericAIController` (`AIBlueprintHelperLibrary.GetAIController` _array_element)))
    (`/Game/GameContent/Gameplay/Elements/Enemies/Base/BP/BP_GenericAIController.Event Stop` _asbp_generic_aicontroller)))

(fn `RegisterEnemy`
  (params (Enemy :type "/Game/GameContent/Gameplay/Elements/Enemies/Base/BP/BP_BaseEnemy Object Reference"))
  (`KismetArrayLibrary.Array_Add` (`self._spawedEnemies`) Enemy))

(fn `UnregisterEnemy`
  (params (Enemy :type "/Game/GameContent/Gameplay/Elements/Enemies/Base/BP/BP_BaseEnemy Object Reference"))
  (`KismetArrayLibrary.Array_RemoveItem` (`self._spawedEnemies`) Enemy)
  (`self.CheckWaveState`)
  (return))