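; Launcher pawn that fires the player's drone and catches it on landing, registering itself with the game state.
; A state enum gates aim-driven rotation and launching; the player controller's possession passes between launcher and drone.
; Launch unregisters the magnet attractor and retracts the mesh by timeline.
; Deploy raises it and enables magnet and landing collision, whose overlap stops, reattaches and broadcasts the landed drone, readying relaunch.
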(event `self.ReceiveBeginPlay`
  (`|ExecutionSequence`
    (:`then_0`
      (`Controller.Possess` (`GameplayStatics.GetPlayerController` 0) self))
    (:`then_1`
      (bind _returnvalue (`|SpawnActorFromClass` "/Game/GameContent/Gameplay/Elements/Drone/BP/BP_Drone.BP_Drone_C" (`KismetMathLibrary.MakeTransform` (0.0 0.0 0.0)) "AlwaysSpawn" "OverrideRootScale" null null))
      (bind _output_get (set `self.LandedDrone` _returnvalue))
      (`self.K2_AttachToComponent` _output_get (`self.LaunchPosition`) "None" "KeepRelative" "KeepRelative" "KeepRelative" true)
      (set `self.State` "NewEnumerator2"))
    (:`then_2`
      (`/Game/GameContent/Gameplay/Systems/GameStates/BP_GameState.Event Register Launcher` (cast `/Game/GameContent/Gameplay/Systems/GameStates/BP_GameState` (`GameplayStatics.GetGameState`) :!pure true) self)
      (`PrimitiveComponent.SetCollisionEnabled` (`self.COL_LandArea`) "NoCollision"))))

(event `self.ReceiveTick`
  (params (DeltaSeconds :type "Float (single-precision)"))
  (switch `/Game/GameContent/Gameplay/Elements/Launcher/BP/ELauncherState` (`self.State`)
    (:`NewEnumerator1`
      _)
    (:`NewEnumerator2`
      _))
  (`self.RotateToAimDirection`))

(event `InputAction|Action`
  (params (Key :type "Key Structure"))
  (bind _landeddrone (`self.LandedDrone`))
  (:`Pressed`
    (switch `/Game/GameContent/Gameplay/Elements/Launcher/BP/ELauncherState` (`self.State`)
      (:`NewEnumerator2`
        ;[1 1 1] Launch drone and possess it
        (`|ExecutionSequence`
          (:`then_0`
            (`Controller.Possess` (`self.GetController`) _landeddrone)
            (`/Game/GameContent/Gameplay/Elements/Drone/BP/BP_Drone.Launch` _landeddrone (`SceneComponent.GetForwardVector` (`self.DefaultSceneRoot`)))
            (set `self.State` "NewEnumerator0")
            (`/Game/GameContent/Gameplay/Elements/Attractor/Components/BP_AttractorComponent.UnregisterToManager` (`self.MagnetAttractor`)))
          (:`then_1`
            (bind (_direction _interpolator) (`Timeline|Recall Timeline` :!via `PlayFromStart`)
              (:`Update`
                (`SceneComponent.K2_SetRelativeLocation` (`self.SM_Launcher`) (`KismetMathLibrary.VLerp` (0.0 0.0 0.0) (0.0 0.0 -250.0) _interpolator) false false)))))))))

(event `Event Ready To Launch`
  (set `self.State` "NewEnumerator2"))

(event `Event Deploy`
  (bind (_direction _lerpt) (`Timeline|Deploy Timeline` :!via `PlayFromStart`)
    (:`Update`
      (`SceneComponent.K2_SetRelativeLocation` (`self.SM_Launcher`) (`KismetMathLibrary.VLerp` (0.0 0.0 -250.0) (0.0 0.0 0.0) _lerpt) false false))
    (:`Finished`
      (set `self.State` "NewEnumerator3")
      (`/Game/GameContent/Gameplay/Elements/Attractor/Components/BP_AttractorComponent.RegisterToManager` (`self.MagnetAttractor`))
      (`PrimitiveComponent.SetCollisionEnabled` (`self.COL_LandArea`) "QueryOnly"))))

(event `self.COL_LandArea.OnComponentBeginOverlap`
  (params (OverlappedComponent :type "PrimitiveComponent Object Reference") (OtherActor :type "Actor Object Reference") (OtherComp :type "PrimitiveComponent Object Reference") (OtherBodyIndex :type Integer) (bFromSweep :type Boolean) (SweepResult :type "HitResult Structure (by ref)"))
  (bind _launchposition (`self.LaunchPosition`))
  (bind _asbp_drone (cast `/Game/GameContent/Gameplay/Elements/Drone/BP/BP_Drone` OtherActor))
  (`KismetSystemLibrary.PrintString` "Landed Drone" true true (struct :`G` 1.0 :`B` 0.255053 :`A` 1.0))
  (`PrimitiveComponent.SetCollisionEnabled` (`self.COL_LandArea`) "NoCollision")
  ;[1 1 1] Land Drone
  (`/Game/GameContent/Gameplay/Elements/Drone/BP/BP_Drone.Event Stop` _asbp_drone)
  (`self.K2_SetActorLocation` _asbp_drone (`SceneComponent.K2_GetComponentLocation` _launchposition) false true)
  (`self.K2_AttachToComponent` _asbp_drone _launchposition "None" "KeepWorld" "KeepRelative" "KeepRelative" false)
  (`Controller.Possess` (`self.GetController` _asbp_drone) self)
  (`self.OnLandDrone`)
  (`self.Event Ready To Launch`))

(fn `RotateToAimDirection`
  (`self.K2_SetActorRotation` (`KismetMathLibrary.MakeRotationFromAxes` (`KismetMathLibrary.Conv_Vector2DToVector` (`/Game/GameContent/Gameplay/Elements/PlayerController/BP_BaseController.GetAimDirection` (cast `/Game/GameContent/Gameplay/Elements/PlayerController/BP_BaseController` (`self.GetController`) :!pure true))) (0.0 0.0 0.0) (0.0 0.0 1.0))))

(fn `UserConstructionScript`)