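; BPC_HeathBar is a health component that tracks current and maximum health for its owner.
; BeginPlay derives starting health from MaxHealth and a start percentage, and SetMaxHealth keeps the maximum at least 1 and clamps current health to it.
; TakeDamages floors health at zero, fires damage and death callbacks, and returns whether health is depleted.
; RecupLife fires a recovery callback but caps the result at CurrentHealth instead of MaxHealth, so health never rises.
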(event `self.ReceiveBeginPlay`
  (set `self._currentHealth` (`KismetMathLibrary.FTrunc` (* (`KismetMathLibrary.Conv_IntToDouble` (`self.MaxHealth`)) (`self.StartHealthPercentage`)))))

(fn `GetCurrentHealth`
  (returns (Health :type Integer))
  (return (`self._currentHealth`)))

(fn `GetMaxHealth`
  (returns (`Max Health` :type Integer))
  (return (`self.MaxHealth`)))

(fn `RecupLife`
  (params (Points :type Integer :default 20))
  (set `self._currentHealth` (`KismetMathLibrary.Min` (+ Points (`self._currentHealth`)) (`self._currentHealth`)))
  (`self.OnRecupLife` Points))

(fn `SetMaxHealth`
  (params (`New Max Health` :type Integer :default 300))
  (bind _output_get (set `self.MaxHealth` (`KismetMathLibrary.Max` `New Max Health` 1)))
  (set `self._currentHealth` (`KismetMathLibrary.Min` _output_get (`self._currentHealth`))))

(fn `TakeDamages`
  (params (Damages :type Integer :default 10))
  (returns (IsDead :type Boolean))
  (bind _output_get (set `self._currentHealth` (`KismetMathLibrary.Max` (- (`self._currentHealth`) Damages))))
  (`self.OnTakeDamages` Damages)
  (`|ExecutionSequence`
    (:`then_0`
      (bind _returnvalue (<= _output_get 0))
      (if _returnvalue
        (`self.OnDie`)))
    (:`then_1`
      (return _returnvalue))))