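; BP_GameState coordinates the round loop and loss condition between the launcher, enemies manager, towers manager and game mode.
; When the enemies manager ends a round, the registered launcher deploys, and its drone-landing callback starts the next round after a short delay.
; When the towers manager reports no towers left, it recalls all enemies and triggers the lose event on BP_BaseMode.
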(event `Event Round Start`)

(event `self.EnemiesManager.OnRoundOver`
  (`/Game/GameContent/Gameplay/Elements/Launcher/BP/BP_Launcher.Event Deploy` (`self.Launcher`)))

(event `Event Register Launcher`
  (params (Launcher :type "/Game/GameContent/Gameplay/Elements/Launcher/BP/BP_Launcher Object Reference"))
  (bind _output_get (set `self.Launcher` Launcher))
  (add `/Game/GameContent/Gameplay/Elements/Launcher/BP/BP_Launcher.OnLandDrone` _output_get (delegate `Event Land Drone`)))

(event `Event Land Drone`
  (`KismetSystemLibrary.Delay` 0.2)
  (`/Game/GameContent/Gameplay/Elements/Enemies/Base/BP/BP_EnemiesManager.Event Start Round` (`self.EnemiesManager`)))

(event `self.TowersManager.OnTowersEmpty`
  (`/Game/GameContent/Gameplay/Elements/Enemies/Base/BP/BP_EnemiesManager.RecallAllEnemies` (`self.EnemiesManager`))
  (`/Game/GameContent/Gameplay/Systems/Modes/BP_BaseMode.Event Lose` (cast `/Game/GameContent/Gameplay/Systems/Modes/BP_BaseMode` (`GameplayStatics.GetGameMode`) :!pure true)))

(fn `UserConstructionScript`)